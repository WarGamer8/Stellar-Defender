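; Player camera character that flies around the level and handles tower selection and placement.
; Enhanced Input drives movement and scrolling, with a toggle that switches between mouse-look and cursor-driven UI.
; SpawnTowerToPlace spawns a preview tower that Tick eases along the deprojected mouse ray at a scroll-adjusted distance until left click places it.
; It also creates the tower sidebar and stat widgets and briefly shows a not-enough-Star-Dust warning.
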(event Custom|SpawnTowerToPlace
  (params (TowerToSpawn :type Actor%20Class%20Reference))
  (bind _maincamera (Variables|Default|GetMainCamera))
  (bind _returnvalue (Transformation|GetWorldTransform _maincamera))
  (Development|PrintString (Utilities|GetClassDisplayName TowerToSpawn))
  (Utilities|IsValid (Variables|Default|GetTowerToPlace)
    (:Is%20Valid
      (Actor|DestroyActor (Variables|Default|GetTowerToPlace)))
    (:Is%20Not%20Valid
      _))
  (bind _returnvalue_2 (Game|SpawnActorfromClass TowerToSpawn (Math|Transform|MakeTransform (+ (* (Math|Vector|GetForwardVector _maincamera) (Variables|Default|GetTowerPlacmentScroll)) (.location _returnvalue)) (.rotation _returnvalue) (.scale _returnvalue)) "AlwaysSpawn" "MultiplyWithRoot" 0 0))
  (Development|PrintString (Utilities|GetDisplayName _returnvalue_2))
  (bind _astower (Utilities|Casting|CastToTower _returnvalue_2))
  (Variables|/Game/Towers/Tower.Tower_C|SetCameraCharacter _astower self)
  (Variables|Default|SetTowerToPlace _astower))

(event Custom|NotEnoughStarDust
  (bind _nodustwidget (Variables|Default|GetNoDustWidget))
  (UserInterface|Viewport|AddtoViewport _nodustwidget 0)
  (Utilities|FlowControl|Delay 2.0)
  (Widget|RemovefromParent _nodustwidget))

(event Input|EnhancedActionEvents|EnhancedInputActionIA_MouseMovmentX
  (params (ActionValue :type Float%20%28double-precision%29) (ElapsedSeconds :type Float%20%28double-precision%29) (TriggeredSeconds :type Float%20%28double-precision%29) (InputAction :type Input%20Action%20Object%20Reference :default "/Game/Input/IA_MouseMovmentX.IA_MouseMovmentX"))
  ;[0.15 0.15 0.15 0.5] Camera Rotation
  (if (Variables|Default|GetRotateCamera)
    (Pawn|Input|AddControllerYawInput ActionValue)))

(event Input|EnhancedActionEvents|EnhancedInputActionIA_MouseMovmentY
  (params (ActionValue :type Float%20%28double-precision%29) (ElapsedSeconds :type Float%20%28double-precision%29) (TriggeredSeconds :type Float%20%28double-precision%29) (InputAction :type Input%20Action%20Object%20Reference :default "/Game/Input/IA_MouseMovmentY.IA_MouseMovmentY"))
  ;[0.15 0.15 0.15 0.5] Camera Rotation
  (if (Variables|Default|GetRotateCamera)
    (Pawn|Input|AddControllerPitchInput ActionValue)))

(event Input|EnhancedActionEvents|EnhancedInputActionIA_RotateCamera
  (params (ActionValue :type Boolean) (ElapsedSeconds :type Float%20%28double-precision%29) (TriggeredSeconds :type Float%20%28double-precision%29) (InputAction :type Input%20Action%20Object%20Reference :default "/Game/Input/IA_RotateCamera.IA_RotateCamera"))
  (bind _playercontroller (Variables|Default|GetPlayerController))
  ;[0.15 0.15 0.15 0.5] Camera Rotation
  (Variables|/Script/Engine.PlayerController|SetbShowMouseCursor _playercontroller (Variables|Default|GetRotateCamera))
  (bind _output_get (Variables|Default|SetRotateCamera (not (Variables|Default|GetRotateCamera))))
  (if _output_get
    (Input|SetInputModeGameOnly _playercontroller false)
    (else
      (Input|SetInputModeGameandUI _playercontroller 0 "DoNotLock" true false))))

(event Input|EnhancedActionEvents|EnhancedInputActionIA_MoveForward
  (params (ActionValue :type Float%20%28double-precision%29) (ElapsedSeconds :type Float%20%28double-precision%29) (TriggeredSeconds :type Float%20%28double-precision%29) (InputAction :type Input%20Action%20Object%20Reference :default "/Game/Input/IA_MoveForward.IA_MoveForward"))
  ;[0.15 0.15 0.15 0.5] Movement
  (Pawn|Input|AddMovementInput (Math|Vector|GetForwardVector (Variables|Default|GetMainCamera)) (* ActionValue (Utilities|Time|GetWorldDeltaSeconds) 1e+03) false))

(event Input|EnhancedActionEvents|EnhancedInputActionIA_MoveRight
  (params (ActionValue :type Float%20%28double-precision%29) (ElapsedSeconds :type Float%20%28double-precision%29) (TriggeredSeconds :type Float%20%28double-precision%29) (InputAction :type Input%20Action%20Object%20Reference :default "/Game/Input/IA_MoveRight.IA_MoveRight"))
  ;[0.15 0.15 0.15 0.5] Movement
  (Pawn|Input|AddMovementInput (Math|Vector|GetRightVector (Variables|Default|GetMainCamera)) (* ActionValue (Utilities|Time|GetWorldDeltaSeconds) 1e+03) false))

(event Input|EnhancedActionEvents|EnhancedInputActionIA_Scroll
  (params (ActionValue :type Float%20%28double-precision%29) (ElapsedSeconds :type Float%20%28double-precision%29) (TriggeredSeconds :type Float%20%28double-precision%29) (InputAction :type Input%20Action%20Object%20Reference :default "/Game/Input/IA_Scroll.IA_Scroll"))
  (Variables|Default|SetTowerPlacmentScroll (+ ActionValue (Variables|Default|GetTowerPlacmentScroll))))

(event Input|EnhancedActionEvents|EnhancedInputActionIA_LeftClick
  (params (ActionValue :type Boolean) (ElapsedSeconds :type Float%20%28double-precision%29) (TriggeredSeconds :type Float%20%28double-precision%29) (InputAction :type Input%20Action%20Object%20Reference :default "/Game/Input/IA_LeftClick.IA_LeftClick"))
  (Utilities|IsValid (Variables|Default|GetTowerToPlace)
    (:Is%20Valid
      (Default|Place (Variables|Default|GetTowerToPlace))
      (Variables|/Game/Towers/Tower.Tower_C|SetTowerIsPlaced (Variables|Default|GetTowerToPlace) true)
      (Variables|Default|SetTowerToPlace 0))))

(event Input|EnhancedActionEvents|EnhancedInputActionIA_MoveUp
  (params (ActionValue :type Boolean) (ElapsedSeconds :type Float%20%28double-precision%29) (TriggeredSeconds :type Float%20%28double-precision%29) (InputAction :type Input%20Action%20Object%20Reference :default "/Game/Input/IA_MoveUp.IA_MoveUp"))
  (Pawn|Input|AddMovementInput (Math|Vector|GetForwardVector (Variables|Default|GetUpArrow)) (* 1.0 (Utilities|Time|GetWorldDeltaSeconds) 1e+03) false))

(event Input|EnhancedActionEvents|EnhancedInputActionIA_MoveDown
  (params (ActionValue :type Boolean) (ElapsedSeconds :type Float%20%28double-precision%29) (TriggeredSeconds :type Float%20%28double-precision%29) (InputAction :type Input%20Action%20Object%20Reference :default "/Game/Input/IA_MoveDown.IA_MoveDown"))
  (Pawn|Input|AddMovementInput (Math|Vector|GetForwardVector (Variables|Default|GetDownArrow)) (* -1.0 (Utilities|Time|GetWorldDeltaSeconds) 1e+03) false))

(event EventBeginPlay
  (bind _returnvalue (Game|GetPlayerController 0))
  (Input|AddMappingContext (PlayerController|LocalPlayerSubsystems|GetEnhancedInputLocalPlayerSubsystem _returnvalue) "/Game/Input/IMC_MainCamera.IMC_MainCamera" 0 "(bIgnoreAllPressedKeysUntilRelease=True,bForceImmediately=False,bNotifyUserSettings=False)")
  (Variables|Default|SetPlayerController _returnvalue)
  (bind _returnvalue_2 (UserInterface|CreateWidget "/Game/BluePrints/UI/WBP_TowerSideBar.WBP_TowerSideBar_C" _returnvalue))
  (Variables|/Game/BluePrints/UI/WBP_TowerSideBar.WBP_TowerSideBar_C|SetPlayerController _returnvalue_2 _returnvalue)
  (UserInterface|Viewport|AddtoViewport _returnvalue_2 0)
  (Input|SetInputModeGameandUI _returnvalue _returnvalue_2 "DoNotLock" false false)
  (Variables|/Script/Engine.PlayerController|SetbShowMouseCursor _returnvalue true)
  (bind _returnvalue_3 (UserInterface|CreateWidget "/Game/BluePrints/UI/WBP_StatDisplay.WBP_StatDisplay_C"))
  (Variables|Default|SetStatDisplayWidget _returnvalue_3)
  (bind _returnvalue_4 (UserInterface|CreateWidget "/Game/BluePrints/UI/WBP_NoDust.WBP_NoDust_C"))
  (Variables|Default|SetNoDustWidget _returnvalue_4))

(event EventTick
  (params (DeltaSeconds :type Float%20%28single-precision%29))
  (bind _playercontroller (Variables|Default|GetPlayerController))
  (bind _worlddirection (Game|Player|ConvertMouseLocationToWorldSpace _playercontroller))
  (Utilities|IsValid (Variables|Default|GetTowerToPlace)
    (:Is%20Valid
      (Transformation|SetActorLocationAndRotation (Variables|Default|GetTowerToPlace) (Math|Interpolation|VInterpTo (Transformation|GetActorLocation (Variables|Default|GetTowerToPlace)) (+ (* _worlddirection (Variables|Default|GetTowerPlacmentScroll)) (Transformation|GetWorldLocation (Variables|Default|GetMainCamera))) (Utilities|Time|GetWorldDeltaSeconds) (Variables|Default|GetTowerPlacmentZoomSpeed)) (Math|Rotator|MakeRotfromX _worlddirection)))))

(fn ConstructionScript)