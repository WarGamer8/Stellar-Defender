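; Wave spawner that, on pressing 1, launches a wave of enemies with a credit budget that grows 20% per wave.
; It notifies every BP_SpawnPawn, then spawns enemies at randomly picked spawn pawns, facing BP_Blackhole, subtracting each cost until credits drop below zero.
; RandomEnemy draws class, cost and name from wave-number-tiered enemy lists.
; The wave counter then increments, with debug prints throughout.
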(event Custom|WaveStart
  (bind _outactors (Actor|GetAllActorsOfClass "/Game/Spawn/BP_SpawnPawn.BP_SpawnPawn_C"))
  (for _array_element _outactors
    (Default|StartPawnWave _array_element))
  (bind _output_get (Variables|Default|SetStartOfWaveCredits (* (Variables|Default|GetStartOfWaveCredits) 1.2)))
  (Variables|Default|SetDuringWaveCredits _output_get)
  (while (>= (Variables|Default|GetDuringWaveCredits) 0.0)
    (Development|PrintString (Utilities|String|Append "Wave Number: " (Utilities|String|ToString(Integer) (Variables|Default|GetWaveNumber))) true true "(R=0.041444,G=1.000000,B=0.000000,A=1.000000)" 2e+01)
    (bind (_enemyclass _enemycredit _shouldrerolled _name) (CallFunction|RandomEnemy (Variables|Default|GetWaveNumber)))
    (Development|PrintString (Utilities|String|Append "Spawing Enemy:" _name) true true "(R=0.000000,G=0.660000,B=1.000000,A=1.000000)" 2e+01)
    (Variables|Default|SetDuringWaveCredits (- (Variables|Default|GetDuringWaveCredits) _enemycredit))
    (bind _outactors_2 (Actor|GetAllActorsOfClass "/Game/Spawn/BP_SpawnPawn.BP_SpawnPawn_C"))
    (Development|PrintString (Utilities|GetDisplayName (.OutItem (Utilities|Array|Random _outactors_2))) true true "(R=1.000000,G=0.000000,B=0.778356,A=1.000000)" 2e+01)
    (Game|SpawnActorfromClass _enemyclass (Math|Transform|MakeTransform (.location (Transformation|GetActorTransform (.OutItem (Utilities|Array|Random _outactors_2)))) (Math|Rotator|MakeRotfromX (Math|Vector|GetUnitDirection(Vector) (.location (Transformation|GetActorTransform (.OutItem (Utilities|Array|Random _outactors_2)))) (Transformation|GetActorLocation (Variables|Default|GetBlackHole)))) (.scale (Transformation|GetActorTransform (.OutItem (Utilities|Array|Random _outactors_2))))) "AlwaysSpawn" "MultiplyWithRoot" 0 0)
    (Development|PrintString (Utilities|GetClassDisplayName _enemyclass) true true "(R=1.000000,G=0.831497,B=0.000000,A=1.000000)"))
  (Math|Integer|IncrementInt (Variables|Default|GetWaveNumber)
    (:%20%20
      (Development|PrintString (Utilities|String|Append "Start Credits: " (Utilities|String|ToString(Float) (Variables|Default|GetStartOfWaveCredits)) ", Current Credits: " (Utilities|String|ToString(Float) (Variables|Default|GetDuringWaveCredits))) true true "(R=0.938948,G=1.000000,B=0.896065,A=1.000000)" 2e+01))))

(event EventBeginPlay
  (Input|EnableInput (Game|GetPlayerController 0))
  (bind _returnvalue (Actor|GetActorOfClass "/Game/Planet_System/Blueprints/BP_Blackhole.BP_Blackhole_C"))
  (Variables|Default|SetBlackHole _returnvalue))

(event Input|KeyboardEvents|1
  (params (Key :type Key%20Structure :default "None"))
  (:Pressed
    (Development|PrintString "Hello")
    (CallFunction|WaveStart)))

(fn ConstructionScript)

(fn RandomEnemy
  (params (WaveNumber :type Integer))
  (bind _enemylistw50 (Variables|Default|GetEnemyListW50))
  (bind _enemylistw40 (Variables|Default|GetEnemyListW40))
  (bind _enemylistw30 (Variables|Default|GetEnemyListW30))
  (bind _enemylistw26 (Variables|Default|GetEnemyListW26))
  (bind _enemylistw20 (Variables|Default|GetEnemyListW20))
  (bind _enemylistw10 (Variables|Default|GetEnemyListW10))
  (bind _enemylistw5 (Variables|Default|GetEnemyListW5))
  (bind _enemylistw1 (Variables|Default|GetEnemyListW1))
  (bind _outitem (Utilities|Array|Random _enemylistw1))
  (bind _outitem_2 (Utilities|Array|Random _enemylistw50))
  (bind _outitem_3 (Utilities|Array|Random _enemylistw40))
  (bind _outitem_4 (Utilities|Array|Random _enemylistw30))
  (bind _outitem_5 (Utilities|Array|Random _enemylistw26))
  (bind _outitem_6 (Utilities|Array|Random _enemylistw20))
  (bind _outitem_7 (Utilities|Array|Random _enemylistw10))
  (bind _outitem_8 (Utilities|Array|Random _enemylistw5))
  (if (>= WaveNumber 50)
    (return (.class _outitem_2) (.creditcost _outitem_2) false (.name _outitem_2))
    (elif (>= WaveNumber 40)
      (return (.class _outitem_3) (.creditcost _outitem_3) false (.name _outitem_3))
      (elif (>= WaveNumber 30)
        (return (.class _outitem_4) (.creditcost _outitem_4) false (.name _outitem_4))
        (elif (>= WaveNumber 26)
          (return (.class _outitem_5) (.creditcost _outitem_5) false (.name _outitem_5))
          (elif (>= WaveNumber 20)
            (return (.class _outitem_6) (.creditcost _outitem_6) false (.name _outitem_6))
            (elif (>= WaveNumber 10)
              (return (.class _outitem_7) (.creditcost _outitem_7) false (.name _outitem_7))
              (elif (>= WaveNumber 5)
                (return (.class _outitem_8) (.creditcost _outitem_8) false (.name _outitem_8))
                (else
                  (if (>= WaveNumber 1)
                    _
                    (else
                      _))
                  (return (.class _outitem) (.creditcost _outitem) false (.name _outitem)))))))))))